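; AC_CamBehaviour is an actor component that supplies framing data for a camera following a group of tracked actors, starting with its owner.
; Other code adds or removes tracked actors through functions that guard with a membership check and print coloured debug messages.
; GetCenterPosition averages the tracked locations, and GetBoundingDistance turns the furthest distance from that centre into a zoom distance using a base offset and multiplier.
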(event EventBeginPlay
  (Utilities|Array|Add (Variables|CameraSettings|GetTrackingActors) (Components|GetOwner)))

(event EventTick
  (params (DeltaSeconds :type Float%20%28single-precision%29)))

(fn AddTrackingActor
  (params (ActorToTrack :type Actor%20Object%20Reference))
  (Utilities|IsNotTrackingActor ActorToTrack
    (:then
      (Utilities|Array|Add (Variables|CameraSettings|GetTrackingActors) ActorToTrack)
      (Utilities|DebugMessage "Tracking Actor Added!" ActorToTrack false)
      (return))
    (:else
      (Utilities|DebugMessage "Tracking Already Listed" ActorToTrack true))))

(fn RemoveTrackingActor
  (params (ActorToRemove :type Actor%20Object%20Reference))
  (Utilities|IsNotTrackingActor ActorToRemove
    (:then
      (Utilities|DebugMessage "Not Valid Tracking Actor, Unable To Remove! " ActorToRemove true))
    (:else
      (bind _returnvalue (Utilities|Array|RemoveItem (Variables|CameraSettings|GetTrackingActors) ActorToRemove))
      (if _returnvalue
        (Utilities|DebugMessage "Tracking Actor Sucessfully Remove!" ActorToRemove false)
        (else
          (Utilities|DebugMessage "Tracking Actor Not Removed!" 0 true))))))

(fn GetCenterPosition
  (for _array_element (Variables|CameraSettings|GetTrackingActors)
    (Utilities|Array|Add (LocalVariables|GetActorPositions) (Transformation|GetActorLocation _array_element)))
  (return (Math|Vector|GetVectorArrayAverage (LocalVariables|GetActorPositions))))

(fn GetBoundingDistance
  (bind _output_get (LocalVariables|SetArrayLength (Utilities|Array|Length (Variables|CameraSettings|GetTrackingActors))))
  (if (!= _output_get 0)
    (bind _centerpoint (CallFunction|GetCenterPosition))
    (LocalVariables|SetCenterPoint _centerpoint)
    (for _array_element (Variables|CameraSettings|GetTrackingActors)
      (bind _output_get_2 (LocalVariables|SetActorToCenterPointDistance (Math|Vector|Distance(Vector) (Transformation|GetActorLocation _array_element) (LocalVariables|GetCenterPoint))))
      (if (> _output_get_2 (LocalVariables|GetFurthestDistance))
        (LocalVariables|SetFurthestDistance (LocalVariables|GetActorToCenterPointDistance))))
    (return (* (+ (LocalVariables|GetFurthestDistance) (Variables|CameraSettings|GetBaseZoomDistance)) (Variables|CameraSettings|GetZoomMultiplier)))
    (else
      (Utilities|DebugMessage "No Tracking Actors To Calculate BoundingDistance!!!" 0 true))))
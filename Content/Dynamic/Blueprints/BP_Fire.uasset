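; BP_Fire is a fire actor that simulates flickering firelight with three point lights.
; On BeginPlay it starts a Flicker event that loops endlessly, setting each light to a random intensity and then waiting briefly before repeating.
; The main light flickers in a brighter range than the two secondary lights, and the loop runs on a Delay instead of Tick.
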(event Custom|Flicker
  (bind _returnvalue (Math|Random|RandomFloatinRange 6e+01 1e+02))
  (Rendering|Components|Light|SetIntensity (Variables|Default|GetPointLight) (Math|Random|RandomFloatinRange 1e+02 1.4e+02) :!label _label)
  (Rendering|Components|Light|SetIntensity (Variables|Default|GetPointLight2) _returnvalue)
  (Rendering|Components|Light|SetIntensity (Variables|Default|GetPointLight1) _returnvalue)
  (Utilities|FlowControl|Delay 0.2)
  (goto _label))

(event EventBeginPlay
  (CallFunction|Flicker))

(event Collision|EventActorBeginOverlap
  (params (OtherActor :type Actor%20Object%20Reference)))

(event EventTick
  (params (DeltaSeconds :type Float%20%28single-precision%29)))

(fn ConstructionScript)
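; BP_NoBubbleZone is a box trigger volume that forbids bubbles inside it.
; A bubble character entering the box pops after a short delay.
; A body character entering has its Spawnable flag cleared and its sphere hidden with a pop Niagara effect, and leaving the box restores both.
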(event OnComponentBeginOverlap(Box)
  (params (OverlappedComponent :type Primitive%20Component%20Object%20Reference) (OtherActor :type Actor%20Object%20Reference) (OtherComp :type Primitive%20Component%20Object%20Reference) (OtherBodyIndex :type Integer) (bFromSweep :type Boolean) (SweepResult :type Hit%20Result%20Structure%20%28by%20ref%29))
  (bind _asbp_bubble_char (Utilities|Casting|CastToBP_BubbleChar OtherActor)
    (:then
      (Utilities|FlowControl|Delay 0.2)
      (Default|Pop _asbp_bubble_char))
    (:CastFailed
      (bind _asbp_body_char (Utilities|Casting|CastToBP_BodyChar OtherActor))
      (Variables|/Game/Dynamic/Blueprints/Characters/BodyChar/BP_BodyChar.BP_BodyChar_C|SetSpawnable _asbp_body_char false)
      (Rendering|SetVisibility (Variables|/Game/Dynamic/Blueprints/Characters/BodyChar/BP_BodyChar.BP_BodyChar_C|GetSphere _asbp_body_char) false false)
      (Niagara|SpawnSystematLocation "/Game/Dynamic/Blueprints/Characters/BubbleChar/NS_Pop.NS_Pop" (Transformation|GetActorLocation _asbp_body_char))
      (Development|PrintString "POP"))))

(event OnComponentEndOverlap(Box)
  (params (OverlappedComponent :type Primitive%20Component%20Object%20Reference) (OtherActor :type Actor%20Object%20Reference) (OtherComp :type Primitive%20Component%20Object%20Reference) (OtherBodyIndex :type Integer))
  (bind _asbp_body_char (Utilities|Casting|CastToBP_BodyChar OtherActor))
  (Variables|/Game/Dynamic/Blueprints/Characters/BodyChar/BP_BodyChar.BP_BodyChar_C|SetSpawnable _asbp_body_char true)
  (Rendering|SetVisibility (Variables|/Game/Dynamic/Blueprints/Characters/BodyChar/BP_BodyChar.BP_BodyChar_C|GetSphere _asbp_body_char) true false))

(event EventBeginPlay)

(event Collision|EventActorBeginOverlap
  (params (OtherActor :type Actor%20Object%20Reference)))

(event EventTick
  (params (DeltaSeconds :type Float%20%28single-precision%29)))

(fn ConstructionScript)